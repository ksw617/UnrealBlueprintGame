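; Character Blueprint with a basic melee attack and health, using debug prints for overlap enter/exit and death.
; Attack plays a random section of the AM_Attack montage and sets IsAttacking to block repeats until the Hit event clears it.
; Hit runs a debug-drawn forward capsule trace over AttackRange and applies fixed damage to the hit actor.
; Incoming damage lowers HP, clamped at zero, where death is only printed.
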(event `self.ReceiveActorBeginOverlap`
  (params (OtherActor :type "Actor Object Reference"))
  (`KismetSystemLibrary.PrintString` "Enter" true true (struct :`B` 1.0 :`A` 1.0) 10.0 "test1"))

(event `self.ReceiveActorEndOverlap`
  (params (OtherActor :type "Actor Object Reference"))
  (`KismetSystemLibrary.PrintString` "Exit" true true (struct :`R` 1.0 :`A` 1.0) 10.0 "test2"))

(event `Attack`
  (if (not (`self.IsAttacking`))
    (`self.PlayAnimMontage` "/Game/Animations/AM_Attack.AM_Attack" 1.0 (select `int` (`KismetMathLibrary.RandomInteger` 3) :`0` "Attack_A" :`1` "Attack_B" :`2` "Attack_C" :!type "Name"))
    (set `self.IsAttacking` true)))

(event `Hit`
  (bind _returnvalue (`self.K2_GetActorLocation`))
  (set `self.IsAttacking` false)
  (bind _outhit (`KismetSystemLibrary.CapsuleTraceSingle` :`Start` _returnvalue :`End` (+ _returnvalue (* (`self.GetActorForwardVector`) (`self.AttackRange`))) :`Radius` 50.0 :`HalfHeight` 50.0 :`TraceChannel` "TraceTypeQuery3" :`DrawDebugType` "ForDuration"))
  (`GameplayStatics.ApplyDamage` (`.HitActor` (`GameplayStatics.BreakHitResult` _outhit)) 10.0 null self))

(event `self.ReceiveAnyDamage`
  (params (Damage :type "Float (single-precision)") (DamageType :type "DamageType Object Reference") (InstigatedBy :type "Controller Object Reference") (DamageCauser :type "Actor Object Reference"))
  (bind _output_get (set `self.HP` (`KismetMathLibrary.FMax` (- (`self.HP`) Damage))))
  (if (<= _output_get 0.0)
    (`KismetSystemLibrary.PrintString` "Player Death")))

(fn `UserConstructionScript`)